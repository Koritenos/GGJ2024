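; Two-player beat meter actor that registers with the game mode and runs beat lines toward a central KillBox.
; SpawnBeat spawns a BP_MeterLine from each side, one owned by each player character.
; Lines entering the KillBox open the players' input window; leaving it clears every character's fail flag, then hides and destroys the line after a delay.
; InteractLeft tracks overlapping lines, and GetClosestLineToCenter finds the spawned line nearest the KillBox.
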(event `self.KillBox.OnComponentEndOverlap`
  (params (OverlappedComponent :type "PrimitiveComponent Object Reference") (OtherActor :type "Actor Object Reference") (OtherComp :type "PrimitiveComponent Object Reference") (OtherBodyIndex :type Integer))
  (bind _asbp_meter_line (cast `/Game/BeatMeter/BP_MeterLine` OtherActor))
  (bind _outactors (`GameplayStatics.GetAllActorsOfClass` "/Game/ThirdPerson/Blueprints/BP_ThirdPersonCharacter.BP_ThirdPersonCharacter_C"))
  (for _array_element _outactors
    (set `/Game/ThirdPerson/Blueprints/BP_ThirdPersonCharacter.IsFailed` false _array_element)
    (`KismetSystemLibrary.PrintString` "Fail Status Reset")
    (`KismetArrayLibrary.Array_RemoveItem` (`self.LinesInKillBox`) _asbp_meter_line)
    (`self.SetActorHiddenInGame` _asbp_meter_line true)
    (`KismetSystemLibrary.Delay` 1.0)
    (if (`KismetSystemLibrary.IsValid` _asbp_meter_line)
      (`self.K2_DestroyActor` _asbp_meter_line)
      (else
        (`KismetSystemLibrary.PrintString` "Tried to destroy already destroyed meter line")))))

(event `self.KillBox.OnComponentBeginOverlap`
  (params (OverlappedComponent :type "PrimitiveComponent Object Reference") (OtherActor :type "Actor Object Reference") (OtherComp :type "PrimitiveComponent Object Reference") (OtherBodyIndex :type Integer) (bFromSweep :type Boolean) (SweepResult :type "HitResult Structure (by ref)"))
  (bind _asbp_meter_line (cast `/Game/BeatMeter/BP_MeterLine` OtherActor))
  (`KismetArrayLibrary.Array_AddUnique` (`self.LinesInKillBox`) _asbp_meter_line)
  (for _array_element (`self.PlayerCharacters`)
    (`/Game/ThirdPerson/Blueprints/BP_ThirdPersonCharacter.SetInputWindow` _array_element true)))

(event `self.InteractLeft.OnComponentBeginOverlap`
  (params (OverlappedComponent :type "PrimitiveComponent Object Reference") (OtherActor :type "Actor Object Reference") (OtherComp :type "PrimitiveComponent Object Reference") (OtherBodyIndex :type Integer) (bFromSweep :type Boolean) (SweepResult :type "HitResult Structure (by ref)"))
  (bind _asbp_meter_line (cast `/Game/BeatMeter/BP_MeterLine` OtherActor))
  (`KismetArrayLibrary.Array_AddUnique` (`self.LeftActors`) _asbp_meter_line))

(event `self.ReceiveBeginPlay`
  (`KismetSystemLibrary.Delay` 0.1)
  (bind _asbp_third_person_game_mode (cast `/Game/ThirdPerson/Blueprints/BP_ThirdPersonGameMode` (`GameplayStatics.GetGameMode`)))
  (set `/Game/ThirdPerson/Blueprints/BP_ThirdPersonGameMode.BeatMeter` self _asbp_third_person_game_mode)
  (bind _outactors (`GameplayStatics.GetAllActorsOfClass` "/Game/ThirdPerson/Blueprints/BP_ThirdPersonCharacter.BP_ThirdPersonCharacter_C"))
  (set `self.PlayerCharacters` _outactors))

(event `self.InteractLeft.OnComponentEndOverlap`
  (params (OverlappedComponent :type "PrimitiveComponent Object Reference") (OtherActor :type "Actor Object Reference") (OtherComp :type "PrimitiveComponent Object Reference") (OtherBodyIndex :type Integer))
  (bind _asbp_meter_line (cast `/Game/BeatMeter/BP_MeterLine` OtherActor))
  (`KismetArrayLibrary.Array_RemoveItem` (`self.LeftActors`) _asbp_meter_line))

(event `Spawn Beat`
  (if (and (`.bSuccess` (cast `/Game/ThirdPerson/Blueprints/BP_ThirdPersonCharacter` (`GameplayStatics.GetPlayerCharacter` 0) :!pure true)) (`.bSuccess` (cast `/Game/ThirdPerson/Blueprints/BP_ThirdPersonCharacter` (`GameplayStatics.GetPlayerCharacter` 1) :!pure true)))
    (bind _returnvalue (`|SpawnActorFromClass` "/Game/BeatMeter/BP_MeterLine.BP_MeterLine_C" (`SceneComponent.K2_GetComponentToWorld` (`self.RightSpawn`)) "Undefined" "MultiplyWithRoot" null (* (`self.Move Speed`) (0.0 -1.0 0.0)) (`SceneComponent.K2_GetComponentLocation` (`self.KillBox`)) (cast `/Game/ThirdPerson/Blueprints/BP_ThirdPersonCharacter` (`GameplayStatics.GetPlayerCharacter` 0) :!pure true) null))
    (`KismetArrayLibrary.Array_AddUnique` (`self.SpawnedLines`) _returnvalue)
    (bind _returnvalue_2 (`|SpawnActorFromClass` "/Game/BeatMeter/BP_MeterLine.BP_MeterLine_C" (`SceneComponent.K2_GetComponentToWorld` (`self.LeftSpawn`)) "Undefined" "MultiplyWithRoot" null (`self.Move Speed`) (`SceneComponent.K2_GetComponentLocation` (`self.KillBox`)) (cast `/Game/ThirdPerson/Blueprints/BP_ThirdPersonCharacter` (`GameplayStatics.GetPlayerCharacter` 1) :!pure true) null))
    (`KismetArrayLibrary.Array_AddUnique` (`self.SpawnedLines`) _returnvalue_2)))

(fn `GetClosestLineToCenter`
  (returns (`Array Element` :type "/Game/BeatMeter/BP_MeterLine Object Reference"))
  (set `self.CloseTest` 300.0)
  (for _array_element (`self.SpawnedLines`)
    (if (`KismetSystemLibrary.IsValid` _array_element)
      (bind _returnvalue (`KismetMathLibrary.Vector_Distance` (`self.K2_GetActorLocation` _array_element) (`SceneComponent.K2_GetComponentLocation` (`self.KillBox`))))
      (if (< _returnvalue (`self.CloseTest`))
        (set `self.ClosestLine` _array_element)
        (set `self.CloseTest` _returnvalue))))
  (return (`self.ClosestLine`)))

(fn `UserConstructionScript`)