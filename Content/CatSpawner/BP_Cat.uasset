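; Cat actor that shows a named cat sprite with a satisfaction bar and gamepad button prompts, configured from its CatData table row.
; BeginPlay loads the row, and both it and FocusCat shuffle the row's inputs, matching trigger and bumper key names to icons in the CatWidget slots.
; Tick uses a Delay to lower Satisfaction about once a second by the row's decay multiplier, clamps it, and refreshes the bar and sprite.
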(event `FocusCat`
  (bind _uiiterator (`self.UiIterator`))
  (bind (_catname _catsprite _decaymultiplier _perfectscorevalue _inputs) (break `/Game/DataTables/CatStruct` (stale `self.ReceiveBeginPlay` _returnvalue)))
  (`KismetArrayLibrary.Array_Shuffle` _inputs :!label _label)
  (for _array_element _inputs
    (for _array_element_2 (`|MakeArray` (`self.Gamepad Right Trigger`) (`self.Gamepad Left Trigger`) (`self.Gamepad Left Bumper`) (`self.Gamepad Right Bumper`))
      (bind (_texture _name) (break `/Game/CatSpawner/TextureWithMappedName` _array_element_2))
      (if (`KismetStringLibrary.EqualEqual_StrStr` _name (`KismetTextLibrary.Conv_TextToString` (`KismetInputLibrary.Key_GetDisplayName` (`.Key` (break `EnhancedActionKeyMapping` _array_element)))))
        (`KismetSystemLibrary.PrintString` (`KismetStringLibrary.Conv_IntToString` (`self.UiIterator`)))
        (bind _ascat_widget (cast `/Game/CatSpawner/CatWidget` (`WidgetComponent.GetUserWidgetObject` (`self.CatWidget`))))
        (`KismetSystemLibrary.PrintString` (`KismetStringLibrary.Conv_IntToString` _uiiterator) true true (struct :`R` 1.0 :`G` 0.880338 :`B` 0.267789 :`A` 1.0) 8.0)
        (bind _output (`|GetArrayItem` (`|MakeArray` (`/Game/CatSpawner/CatWidget.Input1` _ascat_widget) (`/Game/CatSpawner/CatWidget.Input2` _ascat_widget) (`/Game/CatSpawner/CatWidget.Input3` _ascat_widget) (`/Game/CatSpawner/CatWidget.Input4` _ascat_widget)) _uiiterator))
        (set `Widget.Visibility` "Visible" _output)
        (`Image.SetBrush` _output (make `SlateBrush` "Image" "NoTile" "NoMirror" (struct :`X` 32.0 :`Y` 32.0) (struct) (struct :`SpecifiedColor` (struct :`R` 1.0 :`G` 1.0 :`B` 1.0 :`A` 1.0) :`ColorUseRule` "UseColor_Specified") (struct :`CornerRadii` (struct :`W` 1.0) :`Color` (struct :`SpecifiedColor` (struct) :`ColorUseRule` "UseColor_Specified") :`RoundingType` "HalfHeightRadius") _texture))
        (`/Engine/EditorBlueprintResources/StandardMacros.IncrementInt` (`self.UiIterator`)))))
  (set `self.UiIterator` 0)
  (`PrimitiveComponent.SetCastShadow` (`self.CatWidget`) true)
  (`ProgressBar.SetPercent` (`/Game/CatSpawner/CatWidget.SatisfactionSlider` (stale `self.ReceiveBeginPlay` _ascat_widget)) (`self.Satisfaction`) :!label _label_2)
  (`PaperSpriteComponent.SetSprite` (`self.PaperSprite`) _catsprite))

(event `self.ReceiveTick`
  (params (DeltaSeconds :type "Float (single-precision)"))
  (`|ExecutionSequence`
    (:`then_0`
      ;[1 1 1] Satisfaction decay
      (`KismetSystemLibrary.Delay` 1.0)
      (bind _output_get (set `self.Satisfaction` (- (`self.Satisfaction`) (* (`.DecayMultiplier_8_5659A5E649FEED18FE8E6EA198319309` (break `/Game/DataTables/CatStruct` (stale `self.ReceiveBeginPlay` _returnvalue))) 0.01))))
      (`/Engine/EditorBlueprintResources/StandardMacros.CompareFloat` _output_get 1.0
        (:`>`
          (set `self.Satisfaction` 1.0))
        (:`<`
          (`/Engine/EditorBlueprintResources/StandardMacros.CompareFloat` _output_get
            (:`<`
              (set `self.Satisfaction` 0.0))))))
    (:`then_1`
      (goto _label_2))))

(event `self.ReceiveBeginPlay`
  (bind _returnvalue (`|GetDataTableRow` (`self.CatData`) (`self.CatName`))
    (:`then`
      (bind _ascat_widget (cast `/Game/CatSpawner/CatWidget` (`WidgetComponent.GetUserWidgetObject` (`self.CatWidget`))))
      (`TextBlock.SetText` (`/Game/CatSpawner/CatWidget.CatName` _ascat_widget) (`KismetTextLibrary.Conv_NameToText` (`.CatName_2_52B6736640A99D4126869488E7FB79CB` (break `/Game/DataTables/CatStruct` _returnvalue))))
      (goto _label))))

(fn `UserConstructionScript`)